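; BP_MasterSwitch watches a set of switches and unlocks a door once all of them are unlocked.
; At BeginPlay it binds SwitchOpened to every switch in its Switches array.
; Each time a switch opens, it counts unlocked switches, stopping at the first locked one.
; A full count calls CallOnDoorUnlocked on L1GameState with its DoorId, while a partial count resets to zero.
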(event Custom|SwitchOpened
  (bind _array_element (Utilities|Array|ForEachLoopwithBreak (Variables|Default|GetSwitches) :!label _label)
    (:LoopBody
      (if (Variables|/Game/Blueprints/Actors/Grabbable/Switch/BP_Switch.BP_Switch_C|GetbUnlocked _array_element)
        (Math|Integer|IncrementInt (Variables|Default|GetIndexValue))
        (else
          (goto _label Break))))
    (:Completed
      (if (== (Variables|Default|GetIndexValue) (Utilities|Array|Length (Variables|Default|GetSwitches)))
        (bind _asl1game_state (Utilities|Casting|CastToL1GameState (Game|GetGameState)))
        (Default|CallOnDoorUnlocked _asl1game_state (Variables|Default|GetDoorId))
        (else
          (Variables|Default|SetIndexValue 0))))))

(event EventBeginPlay
  (for _array_element (Variables|Default|GetSwitches)
    (EventDispatchers|BindEventtoSwitchOpened _array_element (EventDispatchers|CreateEvent :!event Custom|SwitchOpened))))

(fn ConstructionScript)