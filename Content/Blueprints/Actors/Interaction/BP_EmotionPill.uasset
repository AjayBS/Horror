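; BP_EmotionPill is an interactable pickup that grants one of four emotions: Anger, Envy, Pride or Greed, chosen by its EmotionState.
; On BeginPlay it sets its static mesh material to match that emotion, using mostly temporary colored floor materials.
; On Interact it sets the matching emotion flag to true on BP_MainGameInstance, then destroys itself.
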(event EventBeginPlay
  (|CallParentFunction)
  (CallFunction|SetMaterialColor))

(event Collision|EventActorBeginOverlap
  (params (OtherActor :type Actor%20Object%20Reference)))

(event EventTick
  (params (DeltaSeconds :type Float%20%28single-precision%29)))

(event EventInteract
  (bind _asbp_main_game_instance (Utilities|Casting|CastToBP_MainGameInstance (Game|GetGameInstance)))
  (switch Utilities|FlowControl|Switch|SwitchonEEmotionsData (Variables|Default|GetEmotionState)
    (:Anger
      (Class|HGGameInstance|SetEmotionValue _asbp_main_game_instance "Anger" true))
    (:Envy
      (Class|HGGameInstance|SetEmotionValue _asbp_main_game_instance "Envy" true))
    (:Pride
      (Class|HGGameInstance|SetEmotionValue _asbp_main_game_instance "Pride" true))
    (:Greed
      (Class|HGGameInstance|SetEmotionValue _asbp_main_game_instance "Greed" true)))
  (Actor|DestroyActor))

(fn ConstructionScript
  (|CallParentFunction))

(fn SetMaterialColor
  (switch Utilities|FlowControl|Switch|SwitchonEEmotionsData (Variables|Default|GetEmotionState)
    (:Anger
      (Rendering|Material|SetMaterial (Variables|Default|GetStaticMesh) 0 "/Engine/EngineDebugMaterials/LevelColorationUnlitMaterial.LevelColorationUnlitMaterial"))
    (:Envy
      (Rendering|Material|SetMaterial (Variables|Default|GetStaticMesh) 0 "/Game/Materials/Floor/M_GreenFloor_Temp.M_GreenFloor_Temp"))
    (:Pride
      (Rendering|Material|SetMaterial (Variables|Default|GetStaticMesh) 0 "/Game/Materials/Floor/M_YellowFloor_Temp.M_YellowFloor_Temp"))
    (:Greed
      (Rendering|Material|SetMaterial (Variables|Default|GetStaticMesh) 0 "/Game/Materials/Floor/M_OrangeFloor_Temp.M_OrangeFloor_Temp"))))