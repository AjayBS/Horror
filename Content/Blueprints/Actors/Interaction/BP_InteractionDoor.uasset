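; BP_InteractionDoor is a hinged door that toggles between open and closed when it receives an Interact event.
; A DoorClosed boolean selects whether the OpenDoorTL timeline plays forward to open or reverses to close.
; The timeline's Alpha drives a Lerp on the relative yaw of StaticMesh1, swinging it a quarter turn.
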(event EventInteract
  (if (Variables|Default|GetbDoorClosed)
    (Variables|Default|SetbDoorClosed false)
    (bind _alpha (Timeline|OpenDoorTL Play)
      (:Update
        (Transformation|SetRelativeRotation (Variables|Default|GetStaticMesh1) (Math|Rotator|MakeRotator 0.0 0.0 (Math|Float|Lerp 0.0 -9e+01 _alpha)) false false)))
    (else
      (Variables|Default|SetbDoorClosed true)
      (Timeline|OpenDoorTL Reverse))))

(fn ConstructionScript
  (|CallParentFunction))