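; An interactable hinged door that always swings away from the player and can start locked until an Unlocked event clears it.
; Interact does nothing while locked; otherwise it toggles between opening and closing.
; On opening, the dot product of the player-to-door direction and the door's forward vector picks the swing side.
; A timeline drives the mesh's yaw toward that side and plays in reverse to close.
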(event EventUnlocked
  (Variables|Default|SetbLocked false))

(event EventInteract
  (bind _self self)
  (if (not (Variables|Default|GetbLocked))
    (if (Variables|Default|GetbDoorClosed)
      (Variables|Default|SetbDoorClosed false)
      (Variables|Default|SetDotProduct (Math|Vector|DotProduct (Math|Vector|Normalize (- (Transformation|GetActorLocation _self) (Transformation|GetActorLocation (Variables|Default|GetPlayerRef)))) (Transformation|GetActorForwardVector _self)))
      (bind _alpha (Timeline|OpenDoorTL PlayFromStart)
        (:Update
          (Transformation|SetRelativeRotation (Variables|Default|GetStaticMesh1) (Math|Rotator|MakeRotator 0.0 0.0 (Math|Float|Lerp 0.0 (Math|Float|SelectFloat 9e+01 -9e+01 (>= (Variables|Default|GetDotProduct) 0.0)) _alpha)) false false)))
      (else
        (Variables|Default|SetbDoorClosed true)
        (Timeline|OpenDoorTL ReverseFromEnd)))))

(fn ConstructionScript
  (|CallParentFunction))