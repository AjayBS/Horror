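; BP_Interaction_Pill is an interactable pill that moves the player to a target point and then hands off to a level loading screen.
; Interact shows a black WBP_LoadingUI, waits out its fade, teleports the pawn, aligns control rotation, disables player actions and switches on the interaction mapping context.
; After a pause, it adds a second loading widget carrying the Level value.
; The construction script applies PillMaterial to the mesh.
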(event EventBeginPlay
  (|CallParentFunction) ; This node is disabled and will not be called.\nDrag off pins to build functionality.
)

(event Collision|EventActorBeginOverlap
  (params (OtherActor :type Actor%20Object%20Reference)))

(event EventTick
  (params (DeltaSeconds :type Float%20%28single-precision%29)))

(event EventInteract
  (bind _targetpoint (Variables|Default|GetTargetPoint))
  (bind _returnvalue (Transformation|GetActorTransform _targetpoint))
  (bind _returnvalue_2 (UserInterface|CreateWidget "/Game/UMG/Essentials/WBP_LoadingUI.WBP_LoadingUI_C" 0 0 "(R=0.000000,G=0.000000,B=0.000000,A=1.000000)"))
  (UserInterface|Viewport|AddtoViewport _returnvalue_2 0)
  (Utilities|FlowControl|Delay (Class|WidgetAnimation|GetEndTime (Variables|/Game/UMG/Essentials/WBP_LoadingUI.WBP_LoadingUI_C|GetFade_On _returnvalue_2)))
  (Transformation|SetActorTransform (Game|Player|GetPlayerPawn 0) _returnvalue false true)
  (Pawn|SetControlRotation (Game|GetPlayerController 0) (.Rotation (Math|Transform|BreakTransform _returnvalue)))
  (CallFunction|DisablePlayerActions)
  (CallFunction|MappingContextforInteracting true)
  (Utilities|FlowControl|Delay 3.0)
  (bind _returnvalue_3 (UserInterface|CreateWidget "/Game/UMG/Essentials/WBP_LoadingUI.WBP_LoadingUI_C" 0 (Variables|Default|GetLevel) "(R=0.000000,G=0.000000,B=0.000000,A=1.000000)"))
  (UserInterface|Viewport|AddtoViewport _returnvalue_3 0))

(fn ConstructionScript
  (|CallParentFunction)
  (Rendering|Material|SetMaterial (Variables|Default|GetStaticMesh) 0 (Variables|Default|GetPillMaterial)))