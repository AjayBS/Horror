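; Yoga mat trigger actor that starts a yoga sequence when the player steps on it while emotions are still locked.
; On box overlap, it checks that the actor is the player character and asks BP_L1GameState whether emotions are unlocked.
; It then messages the game state to swap away from the main character at the mat's transform and create the yoga widget, passing its first beat and four emotion pill variables.
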(event OnComponentBeginOverlap(BoxCollision)
  (params (OverlappedComponent :type Primitive%20Component%20Object%20Reference) (OtherActor :type Actor%20Object%20Reference) (OtherComp :type Primitive%20Component%20Object%20Reference) (OtherBodyIndex :type Integer) (bFromSweep :type Boolean) (SweepResult :type Hit%20Result%20Structure%20%28by%20ref%29))
  (bind _asbp_l1game_state (Utilities|Casting|CastToBP_L1GameState (Game|GetGameState)))
  (bind _returnvalue (Class|L1GameState|IsEmotionsUnlocked _asbp_l1game_state))
  (if (and (== OtherActor (Game|GetPlayerCharacter 0)) (not _returnvalue))
    (CallFunction|SwapCharacter)))

(event EventBeginPlay)

(event Collision|EventActorBeginOverlap
  (params (OtherActor :type Actor%20Object%20Reference)))

(event EventTick
  (params (DeltaSeconds :type Float%20%28single-precision%29)))

(fn ConstructionScript)

(fn SwapCharacter
  (bind _returnvalue (Game|GetGameState))
  (Class|BPIGameStates|SwapCharacter(Message) _returnvalue false (Transformation|GetActorLocation) (Transformation|GetActorRotation))
  (Class|BPIGameStates|CreateYogaWidget(Message) _returnvalue (Variables|Default|GetFirstBeat) (Variables|Default|GetAngerPill) (Variables|Default|GetEnvyPill) (Variables|Default|GetPridePill) (Variables|Default|GetGreedPill)))