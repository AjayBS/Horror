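; Base actor for readable note props that the player can examine up close, with its displayed text set in the construction script.
; An overlap sphere activates per-tick updates that line trace to the player's camera, hiding the prompt when occluded and otherwise rotating it toward the camera.
; Pickup distance toggles the prompt state and the actor's input, letting IA_Action open a note examination widget and call MappingContextForInteracting.
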(event OnComponentBeginOverlap(OverlapSphere)
  (params (OverlappedComponent :type Primitive%20Component%20Object%20Reference) (OtherActor :type Actor%20Object%20Reference) (OtherComp :type Primitive%20Component%20Object%20Reference) (OtherBodyIndex :type Integer) (bFromSweep :type Boolean) (SweepResult :type Hit%20Result%20Structure%20%28by%20ref%29))
  (bind _asbp_player_character (Utilities|Casting|CastToBP_PlayerCharacter OtherActor))
  (Variables|Default|SetPlayerRef _asbp_player_character)
  (Rendering|SetVisibility (Variables|Default|GetPromptWidget) true false)
  (Variables|Default|SetbUpdateActor true))

(event OnComponentEndOverlap(OverlapSphere)
  (params (OverlappedComponent :type Primitive%20Component%20Object%20Reference) (OtherActor :type Actor%20Object%20Reference) (OtherComp :type Primitive%20Component%20Object%20Reference) (OtherBodyIndex :type Integer))
  (Utilities|Casting|CastToBP_PlayerCharacter OtherActor)
  (Rendering|SetVisibility (Variables|Default|GetPromptWidget) false false)
  (Variables|Default|SetbUpdateActor false)
  (Input|DisableInput (Game|GetPlayerController 0)))

(event Input|EnhancedActionEvents|EnhancedInputActionIA_Action
  (params (ActionValue :type Boolean) (ElapsedSeconds :type Float%20%28double-precision%29) (TriggeredSeconds :type Float%20%28double-precision%29) (InputAction :type Input%20Action%20Object%20Reference :default "/Game/Inputs/Actions/IA_Action.IA_Action"))
  (:Started
    (bind _returnvalue (UserInterface|CreateWidget "/Game/UMG/WBP_NoteExamination.WBP_NoteExamination_C"))
    (Class|NoteExaminationWidget|UpdateWidget _returnvalue self)
    (UserInterface|Viewport|AddtoViewport _returnvalue 0)
    (CallFunction|MappingContextforInteracting true)))

(event EventTick
  (params (DeltaSeconds :type Float%20%28single-precision%29))
  (bind _returnvalue (Game|GetPlayerController 0))
  (bind _paper (Variables|Default|GetPaper))
  (bind _promptwidget (Variables|Default|GetPromptWidget))
  (bind _returnvalue_2 (Transformation|GetWorldLocation _paper))
  (Transformation|SetWorldLocation (Variables|Default|GetPromptWidget) (Math|Vector|MakeVector (.x _returnvalue_2) (.y _returnvalue_2) (+ (.z _returnvalue_2) (Variables|Default|GetWidgetDistanceAboveMesh))) false false)
  (if (Variables|Default|GetbUpdateActor)
    (bind (_outhit _returnvalue_3) (Collision|LineTraceByChannel (Transformation|GetActorLocation) (Transformation|GetWorldLocation (Variables|/Script/HorrorScare.L1_Character|GetFollowCamera (Variables|Default|GetPlayerRef))) "TraceTypeQuery1" false 0 "None"))
    (if (not _returnvalue_3)
      (Rendering|SetVisibility _promptwidget true false)
      (Transformation|SetWorldRotation (Variables|Default|GetPromptWidget) (Math|Rotator|FindLookatRotation (Transformation|GetWorldLocation (Variables|Default|GetPromptWidget)) (Transformation|GetWorldLocation (Variables|/Script/HorrorScare.L1_Character|GetFollowCamera (Variables|Default|GetPlayerRef)))) false false)
      (Default|TogglePrompt (.AsWBP%20Pickup%20Prompt (Utilities|Casting|CastToWBP_PickupPrompt (UserInterface|GetUserWidgetObject (Variables|Default|GetPromptWidget)))) (<= (Math|Vector|VectorLength (- (.TraceStart (Collision|BreakHitResult _outhit)) (.TraceEnd (Collision|BreakHitResult _outhit)))) (Variables|Default|GetPickupDistance)))
      (if (<= (Math|Vector|VectorLength (- (.TraceStart (Collision|BreakHitResult _outhit)) (.TraceEnd (Collision|BreakHitResult _outhit)))) (Variables|Default|GetPickupDistance))
        (Input|EnableInput _returnvalue)
        (else
          (Input|DisableInput _returnvalue)))
      (else
        (Rendering|SetVisibility _promptwidget false false)
        (Input|DisableInput (Game|GetPlayerController 0))))))

(fn ConstructionScript
  (Rendering|Components|TextRender|SetText (Variables|Default|GetNoteText) (Variables|Default|GetValue)))