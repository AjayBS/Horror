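; Blueprint library of shared input helpers for gamepad detection and prop interaction.
; IsGamepad reports whether the most recently used hardware device is a gamepad, via the Input Device Subsystem.
; MappingContextForInteracting takes a flag and swaps the first local player's Enhanced Input context between IMC_Default and IMC_InteractProps, adding one and removing the other.
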(fn IsGamepad
  (return (Utilities|Enum|Equal(Enum) (.primarydevicetype (Class|InputDeviceSubsystem|GetMostRecentlyUsedHardwareDevice (|InputDeviceSubsystem))) "Gamepad")))

(fn MappingContextforInteracting
  (params (bInteract :type Boolean))
  (if bInteract
    (Input|AddMappingContext (PlayerController|LocalPlayerSubsystems|GetEnhancedInputLocalPlayerSubsystem (Game|GetPlayerController 0)) "/Game/Inputs/IMC_InteractProps.IMC_InteractProps" 0 "(bIgnoreAllPressedKeysUntilRelease=True,bForceImmediately=False,bNotifyUserSettings=False)")
    (Input|RemoveMappingContext (PlayerController|LocalPlayerSubsystems|GetEnhancedInputLocalPlayerSubsystem (Game|GetPlayerController 0)) "/Game/Inputs/IMC_Default.IMC_Default" "(bIgnoreAllPressedKeysUntilRelease=True,bForceImmediately=False,bNotifyUserSettings=False)")
    (else
      (Input|AddMappingContext (PlayerController|LocalPlayerSubsystems|GetEnhancedInputLocalPlayerSubsystem (Game|GetPlayerController 0)) "/Game/Inputs/IMC_Default.IMC_Default" 0 "(bIgnoreAllPressedKeysUntilRelease=True,bForceImmediately=False,bNotifyUserSettings=False)")
      (Input|RemoveMappingContext (PlayerController|LocalPlayerSubsystems|GetEnhancedInputLocalPlayerSubsystem (Game|GetPlayerController 0)) "/Game/Inputs/IMC_InteractProps.IMC_InteractProps" "(bIgnoreAllPressedKeysUntilRelease=True,bForceImmediately=False,bNotifyUserSettings=False)"))))