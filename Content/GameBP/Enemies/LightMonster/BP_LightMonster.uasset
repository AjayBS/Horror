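; BP_LightMonster is an enemy that tracks how long the player has been facing it.
; IsPlayerLookingAtAI dots the player mesh's forward vector with the direction to the monster, stepping a clamped seen-time counter up or down without any line-of-sight trace.
; Overflowing the counter only prints a debug message.
; GetEQSPoint supplies a NavigationCenterPoint location, apparently for EQS queries; nothing in this file calls either function.
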(event EventBeginPlay)

(fn ConstructionScript)

(fn IsPlayerLookingatAI
  (bind _returnvalue (Game|GetPlayerCharacter 0))
  (bind _returnvalue_2 (Transformation|GetActorLocation))
  (bind _returnvalue_3 (Transformation|GetActorLocation _returnvalue))
  (bind _mesh (Variables|/Script/Engine.Character|GetMesh _returnvalue))
  (bind _returnvalue_4 (Math|Vector|GetForwardVector _mesh))
  (bind _returnvalue_5 (- _returnvalue_2 _returnvalue_3))
  (bind _returnvalue_6 (Math|Vector|Normalize _returnvalue_5))
  (bind _returnvalue_7 (Math|Vector|DotProduct _returnvalue_4 _returnvalue_6))
  (if (and (> _returnvalue_7 0.25) (< _returnvalue_7 1.0))
    (bind _output_get (Variables|Default|SetNoOfSecondsSeen (+ (Variables|Default|GetNoOfSecondsSeen) 0.25)))
    (if (> _output_get 1.0)
      (Variables|Default|SetNoOfSecondsSeen 1.0)
      (Development|PrintString "Looking at me!!"))
    (else
      (bind _output_get_2 (Variables|Default|SetNoOfSecondsSeen (- (Variables|Default|GetNoOfSecondsSeen) 0.25)))
      (if (< _output_get_2 0.0)
        (Variables|Default|SetNoOfSecondsSeen 0.0)))))

(fn GetEQSPoint
  (return (Transformation|GetActorLocation (Variables|Default|GetNavigationCenterPoint))))