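; BP_L1GameState is the Level 1 game state that swaps the player between the main character and the yoga character at a given position and rotation.
; SwapCharacter picks the pawn class for SpawnCharacter, which unpossesses, spawns and possesses the new pawn, then destroys the old one.
; It caches the current pawn from BeginPlay onward and calls MappingContextForInteracting after switching to the yoga character.
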(event EventBeginPlay
  (Variables|Default|SetCurrentPawn (Game|Player|GetPlayerPawn 0)))

(event EventSwapCharacter
  (params (bToMainCharacter :type Boolean) (PositionToSwap :type Vector :default "0, 0, 0") (Rotation :type Rotator :default "0, 0, 0"))
  (if bToMainCharacter
    (CallFunction|SpawnCharacter PositionToSwap Rotation (Variables|Default|GetMainCharacter))
    (else
      (CallFunction|SpawnCharacter PositionToSwap Rotation (Variables|Default|GetYogaCharacter))
      (CallFunction|MappingContextforInteracting true))))

(fn ConstructionScript)

(fn SpawnCharacter
  (params (SpawnTransform_Location :type Vector) (SpawnTransform_Rotation :type Rotator) (PawnToSpawn :type Pawn%20Class%20Reference))
  (Pawn|UnPossess (Game|GetPlayerController 0))
  (bind _returnvalue (Game|SpawnActorfromClass PawnToSpawn (Math|Transform|MakeTransform SpawnTransform_Location SpawnTransform_Rotation "1.000000,1.000000,1.000000") "AdjustIfPossibleButAlwaysSpawn" "MultiplyWithRoot" 0 0))
  (Pawn|Possess (Game|GetPlayerController 0) _returnvalue)
  (Actor|DestroyActor (Variables|Default|GetCurrentPawn))
  (Variables|Default|SetCurrentPawn _returnvalue))