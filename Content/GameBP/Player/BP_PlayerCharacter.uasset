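; First-person player character Blueprint that handles input setup, object interaction and grabbing, crouch capsule resizing, head-bob and weapon visuals.
; Hit results are forwarded to actors through interaction and grab interfaces, keeping the grabbed object for release.
; A timeline lerps capsule height toward the movement component's crouch value and reverses to stand.
; Weapon changes swap one gun mesh's asset and socket, then play an equip montage on the arms.
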(event EventBeginPlay
  (bind _asplayer_controller (Utilities|Casting|CastToPlayerController (Pawn|GetController)))
  (Utilities|IsValid (PlayerController|LocalPlayerSubsystems|GetEnhancedInputLocalPlayerSubsystem _asplayer_controller)
    (:Is%20Valid
      (Input|AddMappingContext (PlayerController|LocalPlayerSubsystems|GetEnhancedInputLocalPlayerSubsystem _asplayer_controller) "/Game/Inputs/IMC_Default.IMC_Default" 0 "(bIgnoreAllPressedKeysUntilRelease=True,bForceImmediately=False,bNotifyUserSettings=False)")
      (Transformation|AttachComponentToComponent (Variables|Default|GetGunMesh) (Variables|Default|GetFirstPersonMesh) "Axe" "KeepRelative" "KeepRelative" "KeepRelative" true))))

(event EventGrabActor
  (params (HitResult :type Hit%20Result%20Structure))
  (bind _hitactor (Collision|BreakHitResult HitResult))
  (bind _output_get (Variables|Default|SetGrabbedObject _hitactor))
  (if (and (Utilities|IsValid _hitactor) (Utilities|DoesObjectImplementInterface _hitactor "/Game/Blueprints/Interfaces/BPI_Grab.BPI_Grab_C"))
    (Class|BPIGrab|GrabObject(Message) _output_get)))

(event EventReleaseActor
  (Utilities|IsValid (Variables|Default|GetGrabbedObject)
    (:Is%20Valid
      (Class|BPIGrab|ReleaseObject(Message) (Variables|Default|GetGrabbedObject))
      (Variables|Default|SetGrabbedObject 0))))

(event EventHitActor
  (params (HitResult :type Hit%20Result%20Structure))
  (bind _hitactor (Collision|BreakHitResult HitResult))
  (if (and (Utilities|IsValid _hitactor) (Utilities|DoesObjectImplementInterface _hitactor "/Game/Blueprints/Interfaces/BPI_Interaction.BPI_Interaction_C"))
    (Class|BPIInteraction|Interact(Message) _hitactor)))

(event EventShortenPlayerCapsule
  (bind _alpha (Timeline|CapsuleTL_Template Play)
    (:Update
      (Components|Capsule|SetCapsuleHalfHeight (Variables|Default|GetCapsuleComponent) (Math|Float|Lerp 88.0 (Variables|/Script/HorrorScare.BPC_Movement|GetCrouchHalfHeight (Variables|Default|GetBPCMovementComponent)) _alpha) true))))

(event EventLengthenPlayerCapsule
  (bind _alpha (Timeline|CapsuleTL_Template Reverse)
    (:Update
      (Components|Capsule|SetCapsuleHalfHeight (Variables|Default|GetCapsuleComponent) (Math|Float|Lerp 88.0 (Variables|/Script/HorrorScare.BPC_Movement|GetCrouchHalfHeight (Variables|Default|GetBPCMovementComponent)) _alpha) true))))

(event EventPlayCameraShake
  (params (bIsSprinting :type Boolean) (MappedValue :type Float%20%28single-precision%29))
  (if bIsSprinting
    (Game|Feedback|ClientStartCameraShake (Game|GetPlayerController 0) "/Game/CameraShakes/CS_HeadBob_Run.CS_HeadBob_Run_C" MappedValue "CameraLocal" "0, 0, 0")
    (else
      (Game|Feedback|ClientStartCameraShake (Game|GetPlayerController 0) "/Game/CameraShakes/CS_HeadBob_Walk.CS_HeadBob_Walk_C" MappedValue "CameraLocal" "0, 0, 0"))))

(event EventWeaponChanged
  (switch Utilities|FlowControl|Switch|SwitchonEWeaponType (Variables|Default|GetCurrentWeapon)
    (:Ak47
      (Components|SkeletalMesh|SetSkeletalMeshAsset (Variables|Default|GetGunMesh) "/Game/Weapons_And_Items/Rifle_-_AK47/SKM_Ak47.SKM_Ak47")
      (Transformation|AttachComponentToComponent (Variables|Default|GetGunMesh) (Variables|Default|GetFirstPersonMesh) "AK47" "KeepRelative" "KeepRelative" "KeepRelative" true)
      (Animation|Montage|PlayMontage (Variables|Default|GetFirstPersonMesh) "/Game/Weapons_And_Items/Rifle_-_AK47/Montages/AM_AK47_CharacterEquip.AM_AK47_CharacterEquip"))
    (:USP
      (Components|SkeletalMesh|SetSkeletalMeshAsset (Variables|Default|GetGunMesh) "/Game/Weapons_And_Items/Pistol_-_USP/SKM_Pistol.SKM_Pistol")
      (Transformation|AttachComponentToComponent (Variables|Default|GetGunMesh) (Variables|Default|GetFirstPersonMesh) "USP_Pistol" "KeepRelative" "KeepRelative" "KeepRelative" true)
      (Animation|Montage|PlayMontage (Variables|Default|GetFirstPersonMesh) "/Game/Weapons_And_Items/Pistol_-_USP/Montages/AM_USP_Character_Equip.AM_USP_Character_Equip"))
    (:Axe
      (Components|SkeletalMesh|SetSkeletalMeshAsset (Variables|Default|GetGunMesh) "/Game/Weapons_And_Items/Melee_-_AX/SKM_Ax.SKM_Ax")
      (Transformation|AttachComponentToComponent (Variables|Default|GetGunMesh) (Variables|Default|GetFirstPersonMesh) "Axe" "KeepRelative" "KeepRelative" "KeepRelative" true)
      (Animation|Montage|PlayMontage (Variables|Default|GetFirstPersonMesh) "/Game/Weapons_And_Items/Melee_-_AX/Montages/AM_Axe_Character_Equip.AM_Axe_Character_Equip"))
    (:FirstAid
      (Components|SkeletalMesh|SetSkeletalMeshAsset (Variables|Default|GetGunMesh) "/Game/Weapons_And_Items/First_Aid_-_Syringe/SKM_Syringe.SKM_Syringe")
      (Transformation|AttachComponentToComponent (Variables|Default|GetGunMesh) (Variables|Default|GetFirstPersonMesh) "FirstAid" "KeepRelative" "KeepRelative" "KeepRelative" true)
      (Animation|Montage|PlayMontage (Variables|Default|GetFirstPersonMesh) "/Game/Weapons_And_Items/First_Aid_-_Syringe/Montages/AM_FirstAid_Character_Equip.AM_FirstAid_Character_Equip"))))

(fn ConstructionScript)