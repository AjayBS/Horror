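; BP_YogaCharacter is a player character for yoga posing that can hand control back to the main character.
; ChangeYogaPose plays a random montage from YogaPoses at double speed, and ResetYogaPose stops the active one instantly.
; An uninterrupted montage end is reported to the GameInstance as the last montage and to the GameState as a successful pose.
; IA_Return requests the GameState swap at the current transform and turns off the interaction mapping context.
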(event Custom|ChangeYogaPose
  (bind _mesh (Variables|Character|GetMesh))
  (bind _returnvalue (Components|SkeletalMesh|GetAnimInstance _mesh))
  (Animation|Montage|MontagePlay _returnvalue (Utilities|Array|Get(acopy) (Variables|Default|GetYogaPoses) (Math|Random|RandomIntegerinRange 0 (- (Utilities|Array|Length (Variables|Default|GetYogaPoses)) 1))) 2.0 "MontageLength" 0.0 true)
  (EventDispatchers|BindEventtoOnMontageEnded _returnvalue (EventDispatchers|CreateEvent :!event Custom|MontageCompleted)))

(event Custom|ResetYogaPose
  (bind _mesh (Variables|Character|GetMesh))
  (bind _returnvalue (Components|SkeletalMesh|GetAnimInstance _mesh))
  (Animation|Montage|MontageStop _returnvalue 0.0 (Animation|Montage|GetCurrentActiveMontage _returnvalue)))

(event Custom|MontageCompleted
  (params (Montage :type Anim%20Montage%20Object%20Reference) (bInterrupted :type Boolean))
  (if (not bInterrupted)
    (Class|BPIGameInstance|SetLastMontage(Message) (Game|GetGameInstance) Montage)
    (Class|BPIGameStates|OnYogaPoseSuccessful(Message) (Game|GetGameState))))

(event Input|EnhancedActionEvents|EnhancedInputActionIA_Return
  (params (ActionValue :type Boolean) (ElapsedSeconds :type Float%20%28double-precision%29) (TriggeredSeconds :type Float%20%28double-precision%29) (InputAction :type Input%20Action%20Object%20Reference :default "/Game/Inputs/Actions/IA_Return.IA_Return"))
  (:Started
    (Class|BPIGameStates|SwapCharacter(Message) (Game|GetGameState) true (Transformation|GetActorLocation) (Transformation|GetActorRotation))
    (CallFunction|MappingContextforInteracting false)))

(fn ConstructionScript)