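; BP_PickupActor_Master is a pickup actor, named as a master, that gives an item and amount to the player's inventory on touch.
; When its Sphere begins overlapping a BP_PlayerCharacter, it calls AddItem on that character's inventory component.
; It destroys itself if the add succeeds with no remainder; otherwise it stores the returned remainder as its new Amount and stays in the world.
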(event OnComponentBeginOverlap(Sphere)
  (params (OverlappedComponent :type Primitive%20Component%20Object%20Reference) (OtherActor :type Actor%20Object%20Reference) (OtherComp :type Primitive%20Component%20Object%20Reference) (OtherBodyIndex :type Integer) (bFromSweep :type Boolean) (SweepResult :type Hit%20Result%20Structure%20%28by%20ref%29))
  (bind _asbp_player_character (Utilities|Casting|CastToBP_PlayerCharacter OtherActor))
  (bind (_remainder _returnvalue) (Class|BPCInventory|AddItem (Variables|/Script/HorrorScare.L1_Character|GetBPCInventoryComponent _asbp_player_character) (Variables|Default|GetItem) (Variables|Default|GetAmount)))
  (if (and _returnvalue (== _remainder 0))
    (Actor|DestroyActor)
    (else
      (Variables|Default|SetAmount (Math|Conversions|ToFloat(Integer) _remainder)))))

(event EventBeginPlay)

(event Collision|EventActorBeginOverlap
  (params (OtherActor :type Actor%20Object%20Reference)))

(event EventTick
  (params (DeltaSeconds :type Float%20%28single-precision%29)))

(fn ConstructionScript)