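; Combination lock prop that the player inspects up close to solve with its BP_LockDial actors.
; Interact blends to the lock camera, freezes movement, swaps to prop input and shows dial arrows; exiting reverses this.
; Arrow widget delegates move a highlight across a two-row, four-column grid, with clicks forwarded through WidgetInteraction for mouse and gamepad.
; CheckEveryTurn tests the code and, on success, plays the opening animation, exits the view and destroys lock and dials.
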(event Custom|ExitLockVIew
  (bind _returnvalue (Game|GetPlayerCharacter 0))
  (bind _returnvalue_2 (Game|GetPlayerController 0))
  (Game|Player|SetViewTargetwithBlend _returnvalue_2 _returnvalue 1.0 "VTBlend_Linear" 0.0 false)
  (Input|DisableInput _returnvalue_2)
  (Input|ResetIgnoreLookInput _returnvalue_2)
  (Variables|/Script/HorrorScare.HG_PlayerController|SetbCanOpenInventory (Variables|Default|GetPlayerController) true)
  (Pawn|Components|CharacterMovement|SetMovementMode (Variables|/Script/Engine.Character|GetCharacterMovement _returnvalue) "MOVE_Walking" 0)
  (Variables|/Script/Engine.PlayerController|SetbShowMouseCursor (Variables|Default|GetPlayerController) false)
  (CallFunction|TurnonVisibilityOfDialArrows false)
  (Input|AddMappingContext (PlayerController|LocalPlayerSubsystems|GetEnhancedInputLocalPlayerSubsystem (Game|GetPlayerController 0)) "/Game/Inputs/IMC_Default.IMC_Default" 0 "(bIgnoreAllPressedKeysUntilRelease=True,bForceImmediately=False,bNotifyUserSettings=False)")
  (Input|RemoveMappingContext (PlayerController|LocalPlayerSubsystems|GetEnhancedInputLocalPlayerSubsystem (Game|GetPlayerController 0)) "/Game/Inputs/IMC_InteractProps.IMC_InteractProps" "(bIgnoreAllPressedKeysUntilRelease=True,bForceImmediately=False,bNotifyUserSettings=False)")
  (CallFunction|UnbindDelegatesforDials))

(event Input|EnhancedActionEvents|EnhancedInputActionIA_Return
  (params (ActionValue :type Boolean) (ElapsedSeconds :type Float%20%28double-precision%29) (TriggeredSeconds :type Float%20%28double-precision%29) (InputAction :type Input%20Action%20Object%20Reference :default "/Game/Inputs/Actions/IA_Return.IA_Return"))
  (:Started
    (CallFunction|ExitLockVIew)))

(event Input|EnhancedActionEvents|EnhancedInputActionIA_LMB
  (params (ActionValue :type Boolean) (ElapsedSeconds :type Float%20%28double-precision%29) (TriggeredSeconds :type Float%20%28double-precision%29) (InputAction :type Input%20Action%20Object%20Reference :default "/Game/Inputs/Actions/IA_LMB.IA_LMB"))
  (bind _widgetinteraction (Variables|Default|GetWidgetInteraction))
  (:Started
    (Class|WidgetInteractionComponent|PressPointerKey _widgetinteraction "LeftMouseButton")
    (Class|WidgetInteractionComponent|PressPointerKey _widgetinteraction "Gamepad_FaceButton_Bottom"))
  (:Completed
    (Class|WidgetInteractionComponent|ReleasePointerKey _widgetinteraction "LeftMouseButton")
    (Class|WidgetInteractionComponent|ReleasePointerKey _widgetinteraction "Gamepad_FaceButton_Bottom")))

(event EventBeginPlay
  (Variables|Default|SetPlayerController (.AsHG%20Player%20Controller (Utilities|Casting|CastToHG_PlayerController (Game|GetPlayerController 0)))))

(event EventInteract
  (bind _playercontroller (Variables|Default|GetPlayerController))
  (Game|Player|SetViewTargetwithBlend (Game|GetPlayerController 0) (Components|GetOwner (Variables|Default|GetCamera)) 1.0 "VTBlend_Linear" 0.0 false)
  (Pawn|Components|CharacterMovement|DisableMovement (Variables|/Script/Engine.Character|GetCharacterMovement (Game|GetPlayerCharacter 0)))
  (Input|SetIgnoreLookInput (Game|GetPlayerController 0) false)
  (Variables|/Script/HorrorScare.HG_PlayerController|SetbCanOpenInventory (Variables|Default|GetPlayerController) false)
  (Utilities|FlowControl|Delay 1.0)
  (Input|EnableInput _playercontroller)
  (Variables|/Script/Engine.PlayerController|SetbShowMouseCursor _playercontroller true)
  (CallFunction|TurnonVisibilityOfDialArrows true)
  (Input|AddMappingContext (PlayerController|LocalPlayerSubsystems|GetEnhancedInputLocalPlayerSubsystem (Game|GetPlayerController 0)) "/Game/Inputs/IMC_InteractProps.IMC_InteractProps" 0 "(bIgnoreAllPressedKeysUntilRelease=True,bForceImmediately=False,bNotifyUserSettings=False)")
  (Input|RemoveMappingContext (PlayerController|LocalPlayerSubsystems|GetEnhancedInputLocalPlayerSubsystem (Game|GetPlayerController 0)) "/Game/Inputs/IMC_Default.IMC_Default" "(bIgnoreAllPressedKeysUntilRelease=True,bForceImmediately=False,bNotifyUserSettings=False)")
  (CallFunction|SetButtonHighlight)
  (CallFunction|BindDelegatesforDials))

(event EventCheckEveryTurn
  (bind _returnvalue (Class|Lock|CheckCode))
  (if _returnvalue
    (Components|Animation|PlayAnimation (Variables|Default|GetLockMesh) "/Game/Props/Locks/LockOpen_Anim.LockOpen_Anim" false)
    (Utilities|FlowControl|Delay 2.0)
    (CallFunction|ExitLockVIew)
    (Utilities|FlowControl|Delay 1.0)
    (Actor|DestroyActor)
    (for _array_element (Variables|Default|GetLockDials)
      (Actor|DestroyActor _array_element))))

(fn ConstructionScript
  (bind _boxcollision (Variables|Default|GetBoxCollision))
  (Components|Box|SetBoxExtent _boxcollision (Variables|Default|GetBoxExtent) true)
  (Transformation|SetRelativeLocation _boxcollision (Variables|Default|GetBoxPosition) false false))

(fn TurnonVisibilityOfDialArrows
  (params (bVisible :type Boolean))
  (for _array_element (Variables|Default|GetLockDials)
    (bind _asbp_lock_dial (Utilities|Casting|CastToBP_LockDial _array_element))
    (Rendering|SetVisibility (Variables|/Game/Props/Locks/BP_LockDial.BP_LockDial_C|GetUpArrow _asbp_lock_dial) bVisible false)
    (Rendering|SetVisibility (Variables|/Game/Props/Locks/BP_LockDial.BP_LockDial_C|GetDownArrow _asbp_lock_dial) bVisible false)))

(fn BindDelegatesforDials
  (for _array_element (Variables|Default|GetLockDials)
    (bind _asbp_lock_dial (Utilities|Casting|CastToBP_LockDial _array_element))
    (Utilities|FlowControl|Sequence
      (:then_0
        (bind _aswbp_arrow (Utilities|Casting|CastToWBP_Arrow (UserInterface|GetUserWidgetObject (Variables|/Game/Props/Locks/BP_LockDial.BP_LockDial_C|GetUpArrow _asbp_lock_dial))))
        (EventDispatchers|BindEventtoOnHorizontalMovementClicked _aswbp_arrow (EventDispatchers|CreateEvent :!event HorizontalButtonClickedonArrow))
        (EventDispatchers|BindEventtoOnVerticalMovementClicked _aswbp_arrow (EventDispatchers|CreateEvent :!event VerticalButtonClickedonArrow))
        (EventDispatchers|BindEventtoExitButtonClicked _aswbp_arrow (EventDispatchers|CreateEvent :!event Custom|ExitLockVIew)))
      (:then_1
        (bind _aswbp_arrow_2 (Utilities|Casting|CastToWBP_Arrow (UserInterface|GetUserWidgetObject (Variables|/Game/Props/Locks/BP_LockDial.BP_LockDial_C|GetDownArrow _asbp_lock_dial))))
        (EventDispatchers|BindEventtoOnHorizontalMovementClicked _aswbp_arrow_2 (EventDispatchers|CreateEvent :!event HorizontalButtonClickedonArrow))
        (EventDispatchers|BindEventtoOnVerticalMovementClicked _aswbp_arrow_2 (EventDispatchers|CreateEvent :!event VerticalButtonClickedonArrow))
        (EventDispatchers|BindEventtoExitButtonClicked _aswbp_arrow_2 (EventDispatchers|CreateEvent :!event Custom|ExitLockVIew))))))

(fn HorizontalButtonClickedonArrow
  (params (bIsLeft :type Boolean) (RowIndex :type Integer) (ColumnIndex :type Integer))
  (CallFunction|SetAllButtonsUnhighlighted)
  (if bIsLeft
    (bind _output_get (LocalVariables|SetLocalIndex (Math|Integer|Clamp(Integer) (- ColumnIndex 1) 0 3)))
    (CallFunction|SetButtonHighlight RowIndex _output_get)
    (else
      (bind _output_get_2 (LocalVariables|SetLocalIndex (Math|Integer|Clamp(Integer) (+ ColumnIndex 1) 0 3)))
      (CallFunction|SetButtonHighlight RowIndex _output_get_2))))

(fn SetAllButtonsUnhighlighted
  (for _array_element (Variables|Default|GetLockDials)
    (bind _asbp_lock_dial (Utilities|Casting|CastToBP_LockDial _array_element))
    (bind _aswbp_arrow (Utilities|Casting|CastToWBP_Arrow (UserInterface|GetUserWidgetObject (Variables|/Game/Props/Locks/BP_LockDial.BP_LockDial_C|GetUpArrow _asbp_lock_dial))))
    (Default|SetButtonUnfocusedStyle _aswbp_arrow)
    (bind _aswbp_arrow_2 (Utilities|Casting|CastToWBP_Arrow (UserInterface|GetUserWidgetObject (Variables|/Game/Props/Locks/BP_LockDial.BP_LockDial_C|GetDownArrow _asbp_lock_dial))))
    (Default|SetButtonUnfocusedStyle _aswbp_arrow_2)))

(fn SetButtonHighlight
  (params (Row :type Integer) (Column :type Integer))
  (bind _array_element (Utilities|Array|ForEachLoopwithBreak (Variables|Default|GetLockDials) :!label _label)
    (:LoopBody
      (bind _asbp_lock_dial (Utilities|Casting|CastToBP_LockDial _array_element))
      (if (== Row 0)
        (bind _aswbp_arrow (Utilities|Casting|CastToWBP_Arrow (UserInterface|GetUserWidgetObject (Variables|/Game/Props/Locks/BP_LockDial.BP_LockDial_C|GetUpArrow _asbp_lock_dial))))
        (if (== (Variables|/Script/HorrorScare.ArrowWidget|GetColumnIndex _aswbp_arrow) Column)
          (Default|SetButtonFocusedStyle _aswbp_arrow)
          (goto _label Break))
        (else
          (bind _aswbp_arrow_2 (Utilities|Casting|CastToWBP_Arrow (UserInterface|GetUserWidgetObject (Variables|/Game/Props/Locks/BP_LockDial.BP_LockDial_C|GetDownArrow _asbp_lock_dial))))
          (if (== (Variables|/Script/HorrorScare.ArrowWidget|GetColumnIndex _aswbp_arrow_2) Column)
            (Default|SetButtonFocusedStyle _aswbp_arrow_2)
            (goto _label Break)))))))

(fn VerticalButtonClickedonArrow
  (params (bIsBottom :type Boolean) (RowIndex :type Integer) (ColumnIndex :type Integer))
  (CallFunction|SetAllButtonsUnhighlighted)
  (if bIsBottom
    (LocalVariables|SetLocalRow 1)
    (else
      (bind _output_get (LocalVariables|SetLocalRow 0))))
  (CallFunction|SetButtonHighlight _output_get ColumnIndex))

(fn UnbindDelegatesforDials
  (for _array_element (Variables|Default|GetLockDials)
    (bind _asbp_lock_dial (Utilities|Casting|CastToBP_LockDial _array_element))
    (Utilities|FlowControl|Sequence
      (:then_0
        (bind _aswbp_arrow (Utilities|Casting|CastToWBP_Arrow (UserInterface|GetUserWidgetObject (Variables|/Game/Props/Locks/BP_LockDial.BP_LockDial_C|GetUpArrow _asbp_lock_dial))))
        (EventDispatchers|UnbindallEventsfromOnHorizontalMovementClicked _aswbp_arrow)
        (EventDispatchers|UnbindallEventsfromOnVerticalMovementClicked _aswbp_arrow)
        (EventDispatchers|UnbindallEventsfromExitButtonClicked _aswbp_arrow))
      (:then_1
        (bind _aswbp_arrow_2 (Utilities|Casting|CastToWBP_Arrow (UserInterface|GetUserWidgetObject (Variables|/Game/Props/Locks/BP_LockDial.BP_LockDial_C|GetDownArrow _asbp_lock_dial))))
        (EventDispatchers|UnbindallEventsfromOnHorizontalMovementClicked _aswbp_arrow_2)
        (EventDispatchers|UnbindallEventsfromOnVerticalMovementClicked _aswbp_arrow_2)
        (EventDispatchers|UnbindallEventsfromExitButtonClicked _aswbp_arrow_2)))))