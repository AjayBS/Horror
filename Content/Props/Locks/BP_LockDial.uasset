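; BP_LockDial is a single rotating dial for a lock, stepped 36 degrees at a time.
; On BeginPlay it binds up and down arrow widgets to itself, each assigned a rotation direction.
; One timeline, played forward or reversed, animates the mesh roll; on finish it wraps the stored angle, calls FindNumber, notifies the lock via CheckEveryTurn and re-enables rotation.
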(event EventBeginPlay
  (bind _aswbp_arrow (Utilities|Casting|CastToWBP_Arrow (UserInterface|GetUserWidgetObject (Variables|Default|GetUpArrow))))
  (Class|ArrowWidget|InitializeWidget _aswbp_arrow self true)
  (bind _aswbp_arrow_2 (Utilities|Casting|CastToWBP_Arrow (UserInterface|GetUserWidgetObject (Variables|Default|GetDownArrow))))
  (Class|ArrowWidget|InitializeWidget _aswbp_arrow_2 self false))

(event Collision|EventActorBeginOverlap
  (params (OtherActor :type Actor%20Object%20Reference)))

(event EventTick
  (params (DeltaSeconds :type Float%20%28single-precision%29)))

(event EventRotateDial
  (bind (_direction _alpha) (Timeline|RotateDialTL PlayFromStart)
    (:Update
      (Transformation|SetRelativeRotation (Variables|Default|GetLockDialMesh) (Math|Rotator|MakeRotator (+ (Variables|Default|GetDialRotation) (Utilities|Select :Index _direction :Forward (Math|Float|Lerp 0.0 36.0 _alpha) :Backward (Math|Float|Lerp -36.0 0.0 _alpha))) 0.0 0.0) false false))
    (:Finished
      (bind _output_get (Variables|Default|SetDialRotation (+ (Variables|Default|GetDialRotation) (Utilities|Select :Index _direction :Forward (Math|Float|Lerp 0.0 36.0 _alpha) :Backward (Math|Float|Lerp -36.0 0.0 _alpha)))))
      (if (>= _output_get 3.6e+02)
        (Variables|Default|SetDialRotation 0.0)
        (Transformation|SetRelativeRotation (Variables|Default|GetLockDialMesh) "0, 0, 0" false false)
        (elif (< (Variables|Default|GetDialRotation) 0.0)
          (bind _output_get_2 (Variables|Default|SetDialRotation (Math|Float|MapRangeClamped (Variables|Default|GetDialRotation) 0.0 -3.6e+02 3.6e+02 0.0)))
          (Transformation|SetRelativeRotation (Variables|Default|GetLockDialMesh) (Math|Rotator|MakeRotator _output_get_2 0.0 0.0) false false)))
      (Class|LockDial|FindNumber)
      (Class|Lock|CheckEveryTurn (Variables|Default|GetLockRef))
      (Variables|Default|SetbCanRotate true))))

(event EventRotateDialBackwards
  (bind (_direction _alpha) (Timeline|RotateDialTL ReverseFromEnd)
    (:Update
      (Transformation|SetRelativeRotation (Variables|Default|GetLockDialMesh) (Math|Rotator|MakeRotator (+ (Variables|Default|GetDialRotation) (Utilities|Select :Index _direction :Forward (Math|Float|Lerp 0.0 36.0 _alpha) :Backward (Math|Float|Lerp -36.0 0.0 _alpha))) 0.0 0.0) false false))
    (:Finished
      (bind _output_get (Variables|Default|SetDialRotation (+ (Variables|Default|GetDialRotation) (Utilities|Select :Index _direction :Forward (Math|Float|Lerp 0.0 36.0 _alpha) :Backward (Math|Float|Lerp -36.0 0.0 _alpha)))))
      (if (>= _output_get 3.6e+02)
        (Variables|Default|SetDialRotation 0.0)
        (Transformation|SetRelativeRotation (Variables|Default|GetLockDialMesh) "0, 0, 0" false false)
        (elif (< (Variables|Default|GetDialRotation) 0.0)
          (bind _output_get_2 (Variables|Default|SetDialRotation (Math|Float|MapRangeClamped (Variables|Default|GetDialRotation) 0.0 -3.6e+02 3.6e+02 0.0)))
          (Transformation|SetRelativeRotation (Variables|Default|GetLockDialMesh) (Math|Rotator|MakeRotator _output_get_2 0.0 0.0) false false)))
      (Class|LockDial|FindNumber)
      (Class|Lock|CheckEveryTurn (Variables|Default|GetLockRef))
      (Variables|Default|SetbCanRotate true))))

(fn ConstructionScript)